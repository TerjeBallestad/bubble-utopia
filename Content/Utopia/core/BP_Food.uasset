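; BP_Food is a food store in Utopia that registers itself as the game mode's Food reference on BeginPlay.
; AddAmount changes the stored amount, refreshes the visuals and returns the amount.
; UpdateMeshes shows the stock level with five meshes, each visible only when the amount exceeds its index.
; Interact only prints the name of the interacting character's AI controller.
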(event EventBeginPlay
  (bind _asbp_utopia_gm (Utilities|Casting|CastToBP_Utopia_GM (Game|GetGameMode)))
  (Variables|/Game/Utopia/core/BP_Utopia_GM.BP_Utopia_GM_C|SetFood _asbp_utopia_gm self))

(event Collision|EventActorBeginOverlap
  (params (OtherActor :type Actor%20Object%20Reference)))

(event EventTick
  (params (DeltaSeconds :type Float%20%28single-precision%29)))

(event EventInteract
  (params (Character :type BP%20Character%20Test%20Object%20Reference))
  (Development|PrintString (Utilities|GetDisplayName (AI|GetAIController Character))))

(fn ConstructionScript)

(fn AddAmount
  (params (Amount :type Integer))
  (bind _output_get (Variables|Default|SetAmount (+ Amount (Variables|Default|GetAmount))))
  (CallFunction|UpdateMeshes)
  (return _output_get))

(fn UpdateMeshes
  (Utilities|FlowControl|Sequence
    (:then_0
      (Development|SetHiddeninGame (Variables|Default|Getmesh1) (>= (Class|KismetSystemLibrary|MakeLiteralInteger 1) (Variables|Default|GetAmount)) false))
    (:then_1
      (Development|SetHiddeninGame (Variables|Default|Getmesh2) (>= (Class|KismetSystemLibrary|MakeLiteralInteger 2) (Variables|Default|GetAmount)) false))
    (:then_2
      (Development|SetHiddeninGame (Variables|Default|Getmesh3) (>= (Class|KismetSystemLibrary|MakeLiteralInteger 3) (Variables|Default|GetAmount)) false))
    (:then_3
      (Development|SetHiddeninGame (Variables|Default|Getmesh4) (>= (Class|KismetSystemLibrary|MakeLiteralInteger 4) (Variables|Default|GetAmount)) false))
    (:then_4
      (Development|SetHiddeninGame (Variables|Default|Getmesh5) (>= (Class|KismetSystemLibrary|MakeLiteralInteger 5) (Variables|Default|GetAmount)) false))))