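; BP_Poop is a poop actor that destroys itself when its Interact event fires.
; On BeginPlay it has about a 10% chance of taking the first material from WaffleMesh as a rare waffle variant, leaving the mesh itself unchanged.
; It also prints a debug random float.
; An older construction-script roll that swaps between waffle and poop meshes is disconnected and never runs.
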(event EventBeginPlay
  (bind _returnvalue (Math|Random|RandomFloat))
  (Development|PrintString (Utilities|String|ToString(Float) _returnvalue))
  (if (> _returnvalue 0.9)
    (Rendering|Material|SetMaterial (Variables|Default|GetStaticMesh) 0 (Rendering|Material|GetMaterial (Variables|Default|GetWaffleMesh) 0))))

(event Collision|EventActorBeginOverlap
  (params (OtherActor :type Actor%20Object%20Reference)))

(event EventTick
  (params (DeltaSeconds :type Float%20%28single-precision%29)))

(event EventInteract
  (params (Character :type BP%20Character%20Test%20Object%20Reference))
  (Actor|DestroyActor))

(fn ConstructionScript)