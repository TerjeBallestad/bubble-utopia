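; BP_Trees is the Utopia tree feature, showing up to five tree meshes according to its Amount and feeding happiness to the game mode.
; On BeginPlay it registers itself as Trees on BP_Utopia_GM and refreshes mesh visibility.
; AddAmount updates the count, re-runs UpdateMeshes and prints a debug value.
; Tick adds one happiness every frame, regardless of how many trees are visible.
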(event EventBeginPlay
  (bind _asbp_utopia_gm (Utilities|Casting|CastToBP_Utopia_GM (Game|GetGameMode)))
  (bind _output_get (Variables|Default|SetAs%20BP%20Utopia%20GM _asbp_utopia_gm))
  (Variables|/Game/Utopia/core/BP_Utopia_GM.BP_Utopia_GM_C|SetTrees _output_get self)
  (CallFunction|UpdateMeshes))

(event EventTick
  (params (DeltaSeconds :type Float%20%28single-precision%29))
  (Default|AddHapiness (Variables|Default|GetAs%20BP%20Utopia%20GM) 1))

(fn ConstructionScript)

(fn UpdateMeshes
  (Utilities|FlowControl|Sequence
    (:then_0
      (Development|SetHiddeninGame (Variables|Default|Gettree1) (>= (Class|KismetSystemLibrary|MakeLiteralInteger) (Variables|Default|GetAmount)) false))
    (:then_1
      (Development|SetHiddeninGame (Variables|Default|Gettree2) (>= (Class|KismetSystemLibrary|MakeLiteralInteger 1) (Variables|Default|GetAmount)) false))
    (:then_2
      (Development|SetHiddeninGame (Variables|Default|Gettree3) (>= (Class|KismetSystemLibrary|MakeLiteralInteger 2) (Variables|Default|GetAmount)) false))
    (:then_3
      (Development|SetHiddeninGame (Variables|Default|Gettree4) (>= (Class|KismetSystemLibrary|MakeLiteralInteger 3) (Variables|Default|GetAmount)) false))
    (:then_4
      (Development|SetHiddeninGame (Variables|Default|Gettree5) (>= (Class|KismetSystemLibrary|MakeLiteralInteger 4) (Variables|Default|GetAmount)) false))))

(fn AddAmount
  (params (Amount :type Integer))
  (bind _output_get (Variables|Default|SetAmount (+ Amount (Variables|Default|GetAmount))))
  (CallFunction|UpdateMeshes)
  (Development|PrintString (Utilities|String|ToString(Integer) (+ Amount (Variables|Default|GetAmount))))
  (return _output_get))