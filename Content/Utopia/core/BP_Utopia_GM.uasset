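; Game mode for Utopia that creates the HUD, enables game-and-UI input with a visible cursor, and tracks a clamped happiness score.
; HUD buttons add to the Food and Trees amounts or spawn test creatures and bushes around the world origin.
; Spawn X and Y come from separate random reachable-point queries, so the combined location is not guaranteed reachable.
; AddHapiness clamps the score and refreshes the HUD display.
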(event Custom|Add%20Food
  (Default|AddAmount (Variables|Default|GetFood) 1))

(event Custom|Add%20Tree
  (Default|AddAmount (Variables|Default|GetTrees) 1))

(event Custom|Add%20Creature
  (bind _returnvalue (Math|Vector|VectorZero))
  (bind _randomlocation (AI|Navigation|GetRandomReachablePointinRadius _returnvalue 2e+03 0 0))
  (Game|SpawnActorfromClass "/Game/Utopia/creatures/BP_Character_Test.BP_Character_Test_C" (Math|Transform|MakeTransform (Math|Vector|MakeVector (.x _randomlocation) (.y _randomlocation) 0.0) "0.000000,90.000000,0.000000" "1.000000,1.000000,1.000000") "Undefined" "MultiplyWithRoot" 0 0))

(event Custom|Add%20Bush
  (bind _returnvalue (Math|Vector|VectorZero))
  (bind _randomlocation (AI|Navigation|GetRandomReachablePointinRadius _returnvalue 2e+03 0 0))
  (Game|SpawnActorfromClass "/Game/Utopia/core/BP_Bush.BP_Bush_C" (Math|Transform|MakeTransform (Math|Vector|MakeVector (.x _randomlocation) (.y _randomlocation) 4.0) "0.000000,0.000000,0.000000" "1.000000,1.000000,1.000000") "Undefined" "MultiplyWithRoot" 0 0))

(event EventBeginPlay
  (bind _returnvalue (Game|GetPlayerController 0))
  (bind _returnvalue_2 (UserInterface|CreateWidget "/Game/Utopia/ui/UW_Hud.UW_Hud_C"))
  (bind _output_get (Variables|Default|SetHUD _returnvalue_2))
  (UserInterface|Viewport|AddtoViewport _output_get 0)
  (Input|SetInputModeGameandUI _returnvalue 0 "DoNotLock" true false)
  (Variables|/Script/Engine.PlayerController|SetbShowMouseCursor _returnvalue true)
  (Default|SetHappiness _output_get (Variables|Default|GetHapiness) 1000)
  (Utilities|FlowControl|Sequence
    (:then_0
      (EventDispatchers|BindEventtoOnClicked (Variables|/Game/Utopia/ui/UW_Hud.UW_Hud_C|GetHayButton _output_get) (delegate Custom|Add%20Food)))
    (:then_1
      (EventDispatchers|BindEventtoOnClicked (Variables|/Game/Utopia/ui/UW_Hud.UW_Hud_C|GetTreeButton _output_get) (delegate Custom|Add%20Tree)))
    (:then_2
      (EventDispatchers|BindEventtoOnClicked (Variables|/Game/Utopia/ui/UW_Hud.UW_Hud_C|GetCreatureButton _output_get) (delegate Custom|Add%20Creature)))
    (:then_3
      (EventDispatchers|AssignOnClicked (Variables|/Game/Utopia/ui/UW_Hud.UW_Hud_C|GetBushButton _output_get) (delegate Custom|Add%20Bush)))))

(fn ConstructionScript)

(fn AddHapiness
  (params (Hapiness :type Integer))
  (bind _output_get (Variables|Default|SetHapiness (Math|Integer|Clamp(Integer) (+ Hapiness (Variables|Default|GetHapiness)) 0 1000)))
  (Default|SetHappiness (Variables|Default|GetHUD) _output_get 1000))