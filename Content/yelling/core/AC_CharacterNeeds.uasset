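; Character needs component that models Bladder, Hunger, Love and Hygiene as values clamped to the 0–1 range.
; UpdateNeed subtracts per-need decay scaled by delta time, and AddNeed applies additive changes, both returning the resulting needs struct.
; BeginPlay and Tick are empty, and the decay-and-CallUpdateNeeds chain is disconnected, so the component does not decay needs on its own.
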(event EventBeginPlay)

(event EventTick
  (params (DeltaSeconds :type Float%20%28single-precision%29)))

(fn UpdateNeed
  (params (Needs :type F%20Character%20Needs%20Structure) (DT :type Float%20%28double-precision%29))
  (bind _decay (Variables|Default|GetDecay))
  (bind _output_get (Variables|Default|SetNeeds (Utilities|Struct|MakeF_CharacterNeeds (Math|Float|Clamp(Float) (- (.bladder Needs) (* (.bladder _decay) DT))) (Math|Float|Clamp(Float) (- (.hunger Needs) (* (.hunger _decay) DT))) (Math|Float|Clamp(Float) (- (.love Needs) (* (.love _decay) DT))) (Math|Float|Clamp(Float) (- (.hygiene Needs) (* (.hygiene _decay) DT))))))
  (return _output_get))

(fn AddNeed
  (params (Needs :type F%20Character%20Needs%20Structure))
  (bind _output_get (Variables|Default|SetNeeds (Utilities|Struct|MakeF_CharacterNeeds (Math|Float|Clamp(Float) (+ (.bladder Needs) (.bladder (Variables|Default|GetNeeds)))) (Math|Float|Clamp(Float) (+ (.hunger Needs) (.hunger (Variables|Default|GetNeeds)))) (Math|Float|Clamp(Float) (+ (.love Needs) (.love (Variables|Default|GetNeeds)))) (Math|Float|Clamp(Float) (+ (.hygiene Needs) (.hygiene (Variables|Default|GetNeeds)))))))
  (return _output_get))