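; BP_Activity is an activity actor with a configurable mesh and an Interact event that receives a Character.
; The construction script applies the Mesh variable to its StaticMesh component.
; Interact and DestinationReached are empty.
; Disconnected prototype logic would move the character to InteractLocation, transformed from local to world space, using simple or AI movement, with a fixed timer firing DestinationReached.
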(event Custom|DestinationReached)

(event EventBeginPlay)

(event Collision|EventActorBeginOverlap
  (params (OtherActor :type Actor%20Object%20Reference)))

(event EventTick
  (params (DeltaSeconds :type Float%20%28single-precision%29)))

(event EventInteract
  (params (Character :type Object%20Object%20Reference)))

(fn ConstructionScript
  (Components|StaticMesh|SetStaticMesh (Variables|Default|GetStaticMesh) (Variables|Default|GetMesh)))