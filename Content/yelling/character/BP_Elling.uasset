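; BP_Elling is the click-to-move player character, with a needs component that reports to the UI.
; Left click traces under the cursor and moves to the hit point with a debug sphere, skipping interactable actors; the interaction call is disconnected.
; Tick derives a moving flag and XY direction from velocity.
; BeginPlay caches the needs UI from GM_Yelling, and CharacterNeeds updates are forwarded to it.
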(event UpdateNeeds(CharacterNeeds)
  (params (Needs :type F%20Character%20Needs%20Structure))
  (Default|UpdateNeeds (Variables|Default|GetUI%20Needs) Needs))

(event EventBeginPlay
  (bind _asgm_yelling (Utilities|Casting|CastToGM_Yelling (Game|GetGameMode)))
  (bind _output_get (Variables|Default|SetGame%20Mode _asgm_yelling))
  (Variables|Default|SetUI%20Needs (Variables|/Game/yelling/GM_Yelling.GM_Yelling_C|GetUI%20Needs _output_get)))

(event EventTick
  (params (DeltaSeconds :type Float%20%28single-precision%29))
  (bind _returnvalue (Game|Player|GetPlayerPawn 0))
  (bind _returnvalue_2 (Transformation|GetVelocity _returnvalue))
  (bind (_x _y) (Math|Vector|BreakVector _returnvalue_2))
  (bind _output_get (Variables|Default|SetIsMoving (> (Math|Vector|VectorLength _returnvalue_2) 2e+01)))
  (if _output_get
    (Variables|Default|SetDirectionality (Math|Vector2D|MakeVector2D _x _y))))

(event Input|MouseEvents|LeftMouseButton
  (params (Key :type Key%20Structure))
  (bind _returnvalue (Game|GetPlayerController 0))
  (bind _hitresult (Game|Player|GetHitResultUnderCursorbyChannel _returnvalue "TraceTypeQuery1" true))
  (:Pressed
    (if (not (Utilities|DoesObjectImplementInterface (.hitactor _hitresult) "/Game/yelling/core/BI_Interactable.BI_Interactable_C"))
      (AI|Navigation|SimpleMovetoLocation _returnvalue (.location _hitresult))
      (Rendering|Debug|DrawDebugSphere (.location _hitresult) 1e+01 12 "(R=1.000000,G=1.000000,B=1.000000,A=1.000000)" 3.0))))

(fn ConstructionScript)